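; Ball Blueprint that the player knocks around and that can explode and respawn at a fixed elevated point.
; When the player overlaps its Sphere, a collapsed graph launches the physics mesh along the player model's forward vector, ignoring mass.
; The Explode event swaps the mesh for a Niagara effect, then after a short delay resets visibility, teleports the actor and pauses physics briefly before re-enabling it.
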(event `self.ReceiveBeginPlay`
  ;[1 0 0.9872] Init
  (bind _returnvalue (`GameplayStatics.GetActorOfClass` "/Game/BluePrints/Player/Player_BP.Player_BP_C"))
  (set `self.Player` _returnvalue))

(event `self.Sphere.OnComponentBeginOverlap`
  (params (OverlappedComponent :type "PrimitiveComponent Object Reference") (OtherActor :type "Actor Object Reference") (OtherComp :type "PrimitiveComponent Object Reference") (OtherBodyIndex :type Integer) (bFromSweep :type Boolean) (SweepResult :type "HitResult Structure (by ref)"))
  ;[0 1 0.2461] add Impulse
  (cast `/Game/BluePrints/Player/Player_BP` OtherActor)
  (`PrimitiveComponent.AddImpulse` (`self.StaticMesh`) (* (`KismetMathLibrary.GetForwardVector` (`SceneComponent.K2_GetComponentRotation` (`/Game/BluePrints/Player/Player_BP.Model` (`self.Player`)))) 3000.0) "None" true))

(event `Explode`
  (bind _niagara (`self.Niagara`))
  (`SceneComponent.SetVisibility` (`self.StaticMesh`) false false)
  (`SceneComponent.SetVisibility` _niagara true false)
  (`NiagaraComponent.ResetSystem` _niagara)
  (`KismetSystemLibrary.Delay` 1.0)
  (`self.ResetPositionAndStyle`))

(event `ResetPositionAndStyle`
  (bind _staticmesh (`self.StaticMesh`))
  (`SceneComponent.SetVisibility` (`self.StaticMesh`) true false)
  (`SceneComponent.SetVisibility` (`self.Niagara`) false false)
  (`self.K2_SetActorLocation` (0.0 0.0 2750.500488) false true)
  (`PrimitiveComponent.SetSimulatePhysics` _staticmesh false)
  (`KismetSystemLibrary.Delay` 3.0)
  (`PrimitiveComponent.SetSimulatePhysics` _staticmesh true))

(fn `UserConstructionScript`)