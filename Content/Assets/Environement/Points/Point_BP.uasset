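; Point_BP is a floating pickup that the player collects for a mega point.
; Tick spins the mesh and bobs it vertically through a timeline.
; Sphere overlap with Player_BP checks CanPickPoint, then calls AddMegaPoint and the Apparition event.
; Apparition, also run on BeginPlay, hides the mesh and disables collision, restoring both after a one-second delay, despite the macro's "10s" name.
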(event `self.ReceiveBeginPlay`
  ;[1 1 1] Init
  (`self.Apparition`))

(event `self.ReceiveTick`
  (params (DeltaSeconds :type "Float (single-precision)"))
  (bind _staticmesh (`self.StaticMesh`))
  ;[1 1 1] Event tick
  (`SceneComponent.K2_AddWorldRotation` _staticmesh (struct :`Yaw` 6.0) false false)
  (bind (_direction _newtrack_0) (`Timeline|Timeline_0`)
    (:`Update`
      (`SceneComponent.K2_AddWorldOffset` _staticmesh (`KismetMathLibrary.MakeVector` 0.0 0.0 _newtrack_0) false false))))

(event `self.Sphere.OnComponentBeginOverlap`
  (params (OverlappedComponent :type "PrimitiveComponent Object Reference") (OtherActor :type "Actor Object Reference") (OtherComp :type "PrimitiveComponent Object Reference") (OtherBodyIndex :type Integer) (bFromSweep :type Boolean) (SweepResult :type "HitResult Structure (by ref)"))
  ;[1 1 1] On Point
  (bind _asplayer_bp (cast `/Game/BluePrints/Player/Player_BP` OtherActor))
  (if (`/Game/BluePrints/Player/Player_BP.CanPickPoint` _asplayer_bp)
    (`self.Apparition`)
    (`/Game/BluePrints/Player/Player_BP.Add Mega Point` _asplayer_bp)))

(event `Apparition`
  (bind _sphere (`self.Sphere`))
  ;[1 1 1] Func --> Apparition
  (`SceneComponent.SetVisibility` (`self.StaticMesh`) false false)
  (`PrimitiveComponent.SetCollisionEnabled` _sphere "NoCollision")
  (`KismetSystemLibrary.Delay` 1.0)
  (`SceneComponent.SetVisibility` (`self.StaticMesh`) true false)
  (`PrimitiveComponent.SetCollisionEnabled` _sphere "QueryAndPhysics"))

(fn `UserConstructionScript`)