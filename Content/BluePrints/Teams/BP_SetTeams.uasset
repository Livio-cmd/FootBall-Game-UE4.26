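; BP_SetTeams is a short-lived actor that assigns players to one of two teams based on which trigger they overlap.
; Overlapping the Team1 or Team2 component casts the other actor to Player_BP, sets its Team number and swaps the first PlayerModel material to that team's material.
; The actor destroys itself one second after BeginPlay, so assignment only happens during that brief window.
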(event `self.ReceiveBeginPlay`
  (`KismetSystemLibrary.Delay` 1.0)
  (`self.K2_DestroyActor`))

(event `self.Team 1.OnComponentBeginOverlap`
  (params (OverlappedComponent :type "PrimitiveComponent Object Reference") (OtherActor :type "Actor Object Reference") (OtherComp :type "PrimitiveComponent Object Reference") (OtherBodyIndex :type Integer) (bFromSweep :type Boolean) (SweepResult :type "HitResult Structure (by ref)"))
  (bind _asplayer_bp (cast `/Game/BluePrints/Player/Player_BP` OtherActor))
  (set `/Game/BluePrints/Player/Player_BP.Team` 1 _asplayer_bp)
  (`PrimitiveComponent.SetMaterial` (`/Game/BluePrints/Player/Player_BP.PlayerModel` _asplayer_bp) 0 "/Game/Player_Character/Graphics_Physics/Body_MAT.Body_MAT"))

(event `self.Team 2.OnComponentBeginOverlap`
  (params (OverlappedComponent :type "PrimitiveComponent Object Reference") (OtherActor :type "Actor Object Reference") (OtherComp :type "PrimitiveComponent Object Reference") (OtherBodyIndex :type Integer) (bFromSweep :type Boolean) (SweepResult :type "HitResult Structure (by ref)"))
  (bind _asplayer_bp (cast `/Game/BluePrints/Player/Player_BP` OtherActor))
  (set `/Game/BluePrints/Player/Player_BP.Team` 2 _asplayer_bp)
  (`PrimitiveComponent.SetMaterial` (`/Game/BluePrints/Player/Player_BP.PlayerModel` _asplayer_bp) 0 "/Game/Player_Character/Player_Physics/M_Blue.M_Blue"))

(fn `UserConstructionScript`)